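; ZombieController is the AI controller for zombies, starting the ZombieBT behavior tree on BeginPlay.
; AI perception updates write the successfully-sensed flag to the HasspottedPlayer blackboard key.
; The write only requires player character 0 to be a RunCharacter; the perceived actor itself is never checked.
; Leftover nodes for clearing a timer and resetting a bool never run.
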(event OnTargetPerceptionUpdated(AIPerception)
  (params (Actor :type Actor%20Object%20Reference) (Stimulus :type AI%20Stimulus%20Structure))
  (Variables|Default|SetHasSensed (.bSuccessfullySensed (Utilities|Struct|BreakAIStimulus Stimulus)))
  (Utilities|Casting|CastToRunCharacter (Game|GetPlayerCharacter 0))
  (AI|Components|Blackboard|SetValueasBool (AI|GetBlackboard 0) (Utilities|Name|MakeLiteralName "HasspottedPlayer") (Variables|Default|GetHasSensed)))

(event EventBeginPlay
  (AI|RunBehaviorTree "/Game/Blueprints/AI/ZombieBT.ZombieBT"))

(fn ConstructionScript)