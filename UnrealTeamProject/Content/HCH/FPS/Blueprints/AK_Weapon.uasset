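; AK weapon Blueprint for a first-person shooter, handling firing, ammo and timed reload with sounds and animations.
; Fire traces from the camera with random spread, then from the muzzle to that impact, applying physics and an impulse to hit actors of specific cast types.
; It then spawns an impact actor, randomly adds a second muzzle-located actor as a tracer, and pulses a muzzle light.
; BulletSpeed sets the spread and is copied from Reloadtime.
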(event EventFire
  (if (> (Variables|Default|GetAmmocount) 0)
    (CallFunction|AmmoCheck)
    (bind (_returnvalue _impactpoint) (CallFunction|LineTrace))
    (CallFunction|SpawndecalTracer _returnvalue _impactpoint _impactpoint)
    (Utilities|MuzzleFlash)
    (else
      (Audio|PlaySoundatLocation 0 (Transformation|GetWorldLocation (Variables|Default|GetFirstPersonCamera (.AsRun%20Character (Utilities|Casting|CastTo (Game|GetPlayerCharacter 0))))) "0, 0, 0" 1.0 1.0 0.0 0 0 0))))

(event EventReload
  (Components|Animation|PlayAnimation (Variables|Default|GetPrimaryWeapon) 0 false)
  (Utilities|FlowControl|Delay (Variables|Default|GetReloadtime))
  (Variables|Default|SetAmmocount (Variables|Default|GetMaxAnmo)))

(fn ConstructionScript
  (Variables|Default|SetMaxAnmo 30)
  (Variables|Default|SetAmmocount 30)
  (bind _output_get (Variables|Default|SetReloadtime 2.0))
  (Variables|Default|SetBulletSpeed _output_get))

(fn AmmoCheck
  (bind _returnvalue (Math|Random|RandomFloatinRange 0.7 1.2))
  (Math|Integer|DecrementInt (Variables|Default|GetAmmocount)
    (:%20%20
      (Audio|PlaySoundatLocation 0 (Transformation|GetWorldLocation (Variables|Default|GetFirstPersonCamera (.AsRun%20Character (Utilities|Casting|CastTo (Game|GetPlayerCharacter 0))))) "0, 0, 0" (+ _returnvalue 2.5) _returnvalue 0.0 0 0 0)
      (Components|Animation|PlayAnimation (Variables|Default|GetPrimaryWeapon) 0 false))))

(fn LineTrace
  (bind _bulletspeed (Variables|Default|GetBulletSpeed))
  (bind _muzzle (Variables|Default|Getmuzzle))
  (bind _returnvalue (Transformation|GetWorldLocation _muzzle))
  (bind _returnvalue_2 (* _bulletspeed -1.0))
  (bind _asrun_character (Utilities|Casting|CastTo (Game|GetPlayerCharacter 0)))
  (bind _outhit (Collision|LineTraceByChannel (Transformation|GetWorldLocation (Variables|Default|GetFirstPersonCamera _asrun_character)) (+ (+ (* (Math|Vector|GetForwardVector (Variables|Default|GetFirstPersonCamera _asrun_character)) 3e+04) (Transformation|GetWorldLocation (Variables|Default|GetFirstPersonCamera _asrun_character))) (Math|Vector|MakeVector (Math|Random|RandomFloatinRange _returnvalue_2 _bulletspeed) (Math|Random|RandomFloatinRange _returnvalue_2 _bulletspeed) (Math|Random|RandomFloatinRange _returnvalue_2 _bulletspeed))) "TraceTypeQuery1" false 0 "None")) ; Camera Shot
  (bind _outhit_2 (Collision|LineTraceByChannel _returnvalue (.ImpactPoint (Collision|BreakHitResult _outhit)) "TraceTypeQuery1" false 0 "None" true "(R=0.316306,G=1.000000,B=0.238913,A=1.000000)")) ; Guns Shot
  (Utilities|FlowControl|Sequence
    (:then_0
      (bind _aszombiewalk (Utilities|Casting|CastTo (.HitActor (Collision|BreakHitResult _outhit_2))))
      (Physics|SetSimulatePhysics (Variables|/Script/Engine.Character|GetMesh _aszombiewalk) true)
      (Physics|AddImpulse (Variables|/Script/Engine.Character|GetMesh _aszombiewalk) "5000.000000,5000.000000, 0" "None" true)
      (Components|Animation|PlayAnimation (Variables|/Script/Engine.Character|GetMesh _aszombiewalk) 0 false))
    (:then_1
      (bind _asbp_zombie (Utilities|Casting|CastTo (.HitActor (Collision|BreakHitResult _outhit_2))))
      (Physics|SetSimulatePhysics (Variables|/Script/Engine.Character|GetMesh _asbp_zombie) true)
      (Physics|AddImpulse (Variables|/Script/Engine.Character|GetMesh _asbp_zombie) "5000.000000,5000.000000, 0" "None" true)))
  (return _returnvalue (.ImpactPoint (Collision|BreakHitResult _outhit))))

(fn SpawndecalTracer
  (params (Location :type Vector) (SpawnTransForm :type Vector) (Impact :type Vector))
  (Game|SpawnActorfromClass 0 (Math|Transform|MakeTransform SpawnTransForm (Math|Conversions|RotationFromXVector Impact) "0.025000,0.025000,0.025000") "Undefined" 0 0)
  (if (>= (Math|Random|RandomIntegerinRange 1 10) 7)
    (Game|SpawnActorfromClass 0 (Math|Transform|MakeTransform Location (Transformation|GetWorldRotation (Variables|Default|GetFirstPersonCamera (.AsRun%20Character (Utilities|Casting|CastTo (Game|GetPlayerCharacter 0))))) "0.050000,0.050000,0.050000") "Undefined" 0 0))
  (return))