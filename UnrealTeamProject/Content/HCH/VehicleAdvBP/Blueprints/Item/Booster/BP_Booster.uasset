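; BP_Booster is a single-use speed boost pickup for player and AI vehicles.
; When its Box is overlapped, a Sequence tries casts to BP_VehicleBlueprint_AI1 and VehicleBlueprint.
; A matching vehicle gets a fixed forward velocity added to its mesh's physics linear velocity, then the booster destroys itself.
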(event OnComponentBeginOverlap(Box)
  (params (OverlappedComponent :type Primitive%20Component%20Object%20Reference) (OtherActor :type Actor%20Object%20Reference) (OtherComp :type Primitive%20Component%20Object%20Reference) (OtherBodyIndex :type Integer) (bFromSweep :type Boolean) (SweepResult :type Hit%20Result%20Structure%20%28by%20ref%29))
  (Utilities|FlowControl|Sequence
    (:then_0
      (bind _asbp_vehicle_blueprint_ai1 (Utilities|Casting|CastToBP_VehicleBlueprint_AI1 OtherActor))
      (Physics|SetPhysicsLinearVelocity (Variables|/Script/PhysXVehicles.WheeledVehicle|GetMesh _asbp_vehicle_blueprint_ai1) (* (Transformation|GetActorForwardVector _asbp_vehicle_blueprint_ai1) 5e+02) true "None")
      (Actor|DestroyActor))
    (:then_1
      (bind _asvehicle_blueprint (Utilities|Casting|CastToVehicleBlueprint OtherActor))
      (Physics|SetPhysicsLinearVelocity (Variables|/Script/PhysXVehicles.WheeledVehicle|GetMesh _asvehicle_blueprint) (* (Transformation|GetActorForwardVector _asvehicle_blueprint) 5e+02) true "None")
      (Actor|DestroyActor))))

(fn ConstructionScript)