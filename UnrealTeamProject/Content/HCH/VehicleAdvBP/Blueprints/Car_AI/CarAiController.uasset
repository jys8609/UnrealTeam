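; Car AI controller Blueprint drafting spline-following driving; its events and LineTracer are empty, and the driving logic is disconnected.
; GetPath turns a speed-scaled look-ahead point on the first Path actor's spline into a steering value from yaw difference.
; A SpeedLimiter macro gates SetInput throttle and brake.
; The unwired logic brakes above the limit using trace-hit distance, or a separate limit for sharp right corners.
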(event Custom|AICarTick)

(event EventBeginPlay)

(fn ConstructionScript)

(fn SetInput
  (params (Throttle :type Float%20%28single-precision%29) (Brake :type Float%20%28single-precision%29))
  (Class|WheeledVehicleMovementComponent|SetThrottleInput (Variables|Default|GetVehicleMovement) Throttle)
  (Class|WheeledVehicleMovementComponent|SetBrakeInput (Variables|Default|GetVehicleMovement) Brake))

(fn LineTracer)

(fn GetPath
  (params (Array :type Array%20of%20Path%20Object%20References))
  (bind _output (Utilities|Array|Get(acopy) Array))
  (bind _location (Variables|Default|GetLocation))
  (bind _spline (Variables|/Game/VehicleAdvBP/Blueprints/Car_AI/Path.Path_C|GetSpline _output))
  (return (Math|Float|MapRangeClamped (.yaw (Math|Rotator|Delta(Rotator) (Math|Rotator|FindLookatRotation _location (Spline|FindLocationClosesttoWorldLocation _spline (+ (* (Math|Vector|Normalize (Class|SplineComponent|FindTangentClosesttoWorldLocation _spline (Variables|Default|GetLocation) "World")) (Math|Float|MapRangeClamped (Variables|Default|GetCarSpeed) 2e+01 8e+01 5e+01 5e+02)) _location) "World")) (Variables|Default|GetRotation))) -9e+01 9e+01 -1.0 1.0)))