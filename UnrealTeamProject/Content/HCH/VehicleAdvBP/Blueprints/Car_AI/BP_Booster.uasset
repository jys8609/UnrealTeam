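; BP_Booster is a one-shot booster pickup for vehicles that destroys itself on any Box overlap.
; The overlap passes the other actor to Booster1, which casts it to VehicleBlueprint and returns a sum of its movement speed readings plus a large constant.
; The event discards that result and nothing writes to the vehicle, so no boost is applied.
; A failed cast prints a debug string.
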(event OnComponentBeginOverlap(Box)
  (params (OverlappedComponent :type Primitive%20Component%20Object%20Reference) (OtherActor :type Actor%20Object%20Reference) (OtherComp :type Primitive%20Component%20Object%20Reference) (OtherBodyIndex :type Integer) (bFromSweep :type Boolean) (SweepResult :type Hit%20Result%20Structure%20%28by%20ref%29))
  (CallFunction|Booster1 OtherActor)
  (Actor|DestroyActor))

(fn ConstructionScript)

(fn Booster1
  (params (Actor :type Actor%20Object%20Reference))
  (bind _asvehicle_blueprint (Utilities|Casting|CastToVehicleBlueprint Actor)
    (:then
      (return (+ (Class|WheeledVehicleMovementComponent|GetEngineRotationSpeed (Variables|/Script/PhysXVehicles.WheeledVehicle|GetVehicleMovement _asvehicle_blueprint)) (Class|WheeledVehicleMovementComponent|GetForwardSpeed (Variables|/Script/PhysXVehicles.WheeledVehicle|GetVehicleMovement _asvehicle_blueprint)) (Class|MovementComponent|GetMaxSpeed (Variables|/Script/PhysXVehicles.WheeledVehicle|GetVehicleMovement _asvehicle_blueprint)) (Class|MovementComponent|GetModifiedMaxSpeed (Variables|/Script/PhysXVehicles.WheeledVehicle|GetVehicleMovement _asvehicle_blueprint)) 1e+06)))
    (:CastFailed
      (Development|PrintString "Hello"))))