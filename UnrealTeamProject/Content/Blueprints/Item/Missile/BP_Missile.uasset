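; BP_Missile is a projectile that explodes on impact and can home in on racing vehicles.
; A collision hit triggers Bomb once, which fires a radial impulse, spawns the explosion effect, plays a sound and destroys the actor.
; HomingMissile casts the target to the AI or racing vehicle Blueprint, adds a static mesh component to it and makes that the projectile's homing target.
; Disconnected logic that toggles mesh constraint modes never runs.
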(event OnComponentHit(CollisionComponent)
  (params (HitComponent :type Primitive%20Component%20Object%20Reference) (OtherActor :type Actor%20Object%20Reference) (OtherComp :type Primitive%20Component%20Object%20Reference) (NormalImpulse :type Vector :default "0, 0, 0") (Hit :type Hit%20Result%20Structure%20%28by%20ref%29))
  ;[0 0 0] Bomb
  (CallFunction|Bomb))

(event Custom|HomingMissile
  (params (TargetToHit :type Wheeled%20Vehicle%20Object%20Reference))
  (bind _projectile (Variables|MyProjectile|GetProjectile))
  (bind _projectile_2 (Variables|MyProjectile|GetProjectile))
  ;[0 0 0] Set Homing Missile
  (Utilities|FlowControl|Sequence
    (:then_0
      (bind _asbp_vehicle_blueprint_ai1_main (Utilities|Casting|CastToBP_VehicleBlueprint_AI1_Main TargetToHit))
      (bind _returnvalue (AddComponent|AddStaticMeshComponent _asbp_vehicle_blueprint_ai1_main false))
      (if (Utilities|IsValid TargetToHit)
        (Variables|/Script/Engine.ProjectileMovementComponent|SetHomingTargetComponent _projectile_2 _returnvalue)
        (Variables|/Script/Engine.ProjectileMovementComponent|SetbIsHomingProjectile _projectile_2 true)
        (Variables|/Script/Engine.ProjectileMovementComponent|SetHomingAccelerationMagnitude _projectile_2 2.5e+04)))
    (:then_1
      (bind _asvehicle_blueprint_racing (Utilities|Casting|CastToVehicleBlueprint_Racing TargetToHit))
      (bind _returnvalue_2 (AddComponent|AddStaticMeshComponent _asvehicle_blueprint_racing false))
      (if (Utilities|IsValid _asvehicle_blueprint_racing)
        (Variables|/Script/Engine.ProjectileMovementComponent|SetHomingTargetComponent _projectile _returnvalue_2)
        (Variables|/Script/Engine.ProjectileMovementComponent|SetbIsHomingProjectile _projectile true)
        (Variables|/Script/Engine.ProjectileMovementComponent|SetHomingAccelerationMagnitude _projectile 2.5e+04)))))

(event Custom|Bomb
  (bind _explosionforce (Variables|Default|GetExplosionForce))
  ;[0 0 0] Bomb
  (Utilities|FlowControl|DoOnce false
    (:Completed
      (Class|RadialForceComponent|FireImpulse _explosionforce)
      (Effects|SpawnEmitteratLocation "/Game/StarterContent/Particles/P_Explosion.P_Explosion" (Transformation|GetWorldLocation _explosionforce))
      (Audio|PlaySound2D 0 1.0 1.0 0.0 0 0)
      (Actor|DestroyActor))))

(fn ConstructionScript)