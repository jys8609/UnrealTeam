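; AI-driven car that follows a Path spline, managing its own steering, throttle and brake every Tick.
; Steering aims at a spline point found with a speed-scaled look-ahead along the tangent.
; Above a low minimum speed it fires seven line traces and accelerates if the three forward ones are clear.
; On a forward hit, overlapped BP_CornerIndex actors set corner speed limits; outside corners, hits on non-AI1 objects trigger distance-mapped braking.
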(event EventTick
  (params (DeltaSeconds :type Float%20%28single-precision%29))
  (bind _outactors (Actor|GetAllActorsOfClass "/Game/HCH/VehicleAdvBP/Blueprints/Car_AI/Path.Path_C"))
  (bind _steering_amount (CallFunction|GetPath _outactors))
  (Class|WheeledVehicleMovementComponent|SetSteeringInput (Variables|Default|GetVehicleMovement) _steering_amount)
  (Utilities|SpeedLimit 1e+01
    (:Under%20Speed%20Limit
      (CallFunction|SetInput 1.0 0.0))
    (:Over%20Speed%20Limit
      (CallFunction|LineTracer)
      (if (Math|Boolean|ORBoolean (Variables|Hit?|GetFrontLineTraceHit?) (Variables|Hit?|GetLeftFrontOffsetLineTraceHit?) (Variables|Hit?|GetRightFrontOffsetLineTraceHit?))
        (bind _corner (Utilities|GetCorner)
          (:IsInCorner
            (bind _asbp_corner_index (Utilities|Casting|CastToBP_CornerIndex _corner))
            (switch Utilities|FlowControl|Switch|Switchon (Variables|/Game/HCH/VehicleAdvBP/Blueprints/Car_AI/BP_CornerIndex.BP_CornerIndex_C|GetTurnIndex _asbp_corner_index)
              (:NewEnumerator0
                (Utilities|SpeedLimit 3e+01
                  (:Under%20Speed%20Limit
                    (CallFunction|SetInput 1.0 0.0))
                  (:Over%20Speed%20Limit
                    (CallFunction|SetInput 0.0 1.0))))
              (:NewEnumerator1
                (Utilities|SpeedLimit 12.0
                  (:Under%20Speed%20Limit
                    (CallFunction|SetInput 1.0 0.0))
                  (:Over%20Speed%20Limit
                    (CallFunction|SetInput 0.0 1.0))))))
          (:NoInCorner
            (Utilities|CasttoVehicle (Variables|HitResult|GetLeftFrontOffsetLineTraceHitResult)
              (:CastFailed
                (Utilities|CasttoVehicle (Variables|HitResult|GetFrontLineTraceHitResult)
                  (:CastFailed
                    (Utilities|CasttoVehicle (Variables|HitResult|GetRightFrontOffsetLineTraceHitResult)
                      (:CastFailed
                        (CallFunction|SetInput 0.0 (Math|Float|MapRangeClamped (.distance (Utilities|Array|Get(acopy) (Variables|HitResult|GetFrontLineTraceHitResult))) 0.0 1.5e+03 0.0 1.0))))))))))
        (else
          (CallFunction|SetInput 1.0 0.0))))))

(fn ConstructionScript)

(fn GetPath
  (params (Splines :type Array%20of%20Path%20Object%20References))
  (bind _returnvalue (Transformation|GetActorLocation))
  (bind _output (Utilities|Array|Get(acopy) Splines))
  (bind _spline (Variables|/Game/HCH/VehicleAdvBP/Blueprints/Car_AI/Path.Path_C|GetSpline _output))
  (return (Math|Float|MapRangeClamped (.yaw (Math|Rotator|Delta(Rotator) (Math|Rotator|FindLookatRotation _returnvalue (Spline|FindLocationClosesttoWorldLocation _spline (+ (* (Math|Vector|Normalize (Class|SplineComponent|FindTangentClosesttoWorldLocation _spline _returnvalue "World")) (Math|Float|MapRangeClamped (CallFunction|GetCurrentCarSpeed) 2e+01 8e+01 5e+01 5e+02)) _returnvalue) "World")) (Transformation|GetActorRotation))) -9e+01 9e+01 -1.0 1.0)))

(fn GetCurrentCarSpeed
  (return (* (Class|WheeledVehicleMovementComponent|GetForwardSpeed (Variables|Default|GetVehicleMovement)) 0.036)))

(fn SetInput
  (params (Throttle :type Float%20%28single-precision%29) (Brake :type Float%20%28single-precision%29))
  (bind _vehiclemovement (Variables|Default|GetVehicleMovement))
  (Class|WheeledVehicleMovementComponent|SetThrottleInput _vehiclemovement Throttle)
  (Class|WheeledVehicleMovementComponent|SetBrakeInput _vehiclemovement Brake))

(fn LineTracer
  (bind _linetracestartpoint (Variables|Default|GetLineTraceStartPoint))
  (bind _returnvalue (Transformation|GetWorldLocation _linetracestartpoint))
  (for _index (range 0 6)
    (LocalVariables|SetCurrentIndex%28Local%29 _index)
    (bind (_outhits _returnvalue_2) (Class|KismetSystemLibrary|LineTraceMultiforObjects (Utilities|Select :Index (LocalVariables|GetCurrentIndex%28Local%29) :Option%200 _returnvalue :Option%201 _returnvalue :Option%202 (Transformation|GetWorldLocation (Variables|Default|GetLineTreceLeftFrontOffset)) :Option%203 _returnvalue :Option%204 (Transformation|GetWorldLocation (Variables|Default|GetLineTreceRightFrontOffset)) :Option%205 _returnvalue :Option%206 _returnvalue) (+ (Utilities|Select :Index (LocalVariables|GetCurrentIndex%28Local%29) :Option%200 _returnvalue :Option%201 _returnvalue :Option%202 (Transformation|GetWorldLocation (Variables|Default|GetLineTreceLeftFrontOffset)) :Option%203 _returnvalue :Option%204 (Transformation|GetWorldLocation (Variables|Default|GetLineTreceRightFrontOffset)) :Option%205 _returnvalue :Option%206 _returnvalue) (* (Math|Vector|RotateVectorAroundAxis (Math|Vector|GetForwardVector (Variables|Default|GetLineTraceStartPoint)) (Utilities|Select :Index (LocalVariables|GetCurrentIndex%28Local%29) :Option%200 -9e+01 :Option%201 -45.0 :Option%202 0.0 :Option%203 0.0 :Option%204 0.0 :Option%205 45.0 :Option%206 9e+01) "0, 0,1.000000") 1e+03)) (Utilities|Array|MakeArray "ObjectTypeQuery5" "ObjectTypeQuery7") false 0 "None" true))
    (LocalVariables|SetCurrentOutHitResult%20%28Local%29 _outhits)
    (LocalVariables|SetCurrentReturnValue%20%28Local%29 _returnvalue_2)
    (switch int (LocalVariables|GetCurrentIndex%28Local%29)
      (:0
        (Variables|HitResult|SetLeftLineTraceHitResult (LocalVariables|GetCurrentOutHitResult%20%28Local%29))
        (Variables|Hit?|SetLeftLineTraceHit? (LocalVariables|GetCurrentReturnValue%20%28Local%29)))
      (:1
        (Variables|HitResult|SetLeftFrontLineTraceHitResult (LocalVariables|GetCurrentOutHitResult%20%28Local%29))
        (Variables|Hit?|SetLeftFrontLineTraceHit? (LocalVariables|GetCurrentReturnValue%20%28Local%29)))
      (:2
        (Variables|HitResult|SetLeftFrontOffsetLineTraceHitResult (LocalVariables|GetCurrentOutHitResult%20%28Local%29))
        (Variables|Hit?|SetLeftFrontOffsetLineTraceHit? (LocalVariables|GetCurrentReturnValue%20%28Local%29)))
      (:3
        (Variables|HitResult|SetFrontLineTraceHitResult (LocalVariables|GetCurrentOutHitResult%20%28Local%29))
        (Variables|Hit?|SetFrontLineTraceHit? (LocalVariables|GetCurrentReturnValue%20%28Local%29)))
      (:4
        (Variables|HitResult|SetRightFrontOffsetLineTraceHitResult (LocalVariables|GetCurrentOutHitResult%20%28Local%29))
        (Variables|Hit?|SetRightFrontOffsetLineTraceHit? (LocalVariables|GetCurrentReturnValue%20%28Local%29)))
      (:5
        (Variables|HitResult|SetRightFrontLineTraceHitResult (LocalVariables|GetCurrentOutHitResult%20%28Local%29))
        (Variables|Hit?|SetRightFrontLineTraceHit? (LocalVariables|GetCurrentReturnValue%20%28Local%29)))
      (:6
        (Variables|HitResult|SetRightLineTraceHitResult (LocalVariables|GetCurrentOutHitResult%20%28Local%29))
        (Variables|Hit?|SetRightLineTraceHit? (LocalVariables|GetCurrentReturnValue%20%28Local%29)))))
  (return))