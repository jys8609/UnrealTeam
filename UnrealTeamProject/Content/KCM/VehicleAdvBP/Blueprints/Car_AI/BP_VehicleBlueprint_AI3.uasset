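; AI-driven car Blueprint that steers along a Path2 spline and manages its throttle and braking.
; Each tick, steering aims at a spline point projected ahead along the tangent, with lookahead growing with speed.
; Above a minimum speed, a forward trace gates braking: overlapped BP_CornerIndex actors set speed limits for sharp-right and hairpin turns, while hits outside corners brake from hit distance.
; Otherwise it applies full throttle.
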(event EventTick
  (params (DeltaSeconds :type Float%20%28single-precision%29))
  (bind _outactors (Actor|GetAllActorsOfClass "/Game/VehicleAdvBP/Blueprints/Car_AI/Path2.Path2_C"))
  (bind _steering_amount (CallFunction|GetPath _outactors))
  (Class|WheeledVehicleMovementComponent|SetSteeringInput (Variables|Default|GetVehicleMovement) _steering_amount)
  (Utilities|SpeedLimit 1e+01
    (:Under%20Speed%20Limit
      (CallFunction|SetInput 1.0 0.0))
    (:Over%20Speed%20Limit
      (CallFunction|LineTracer)
      (if (Variables|Default|GetFrontLineTraceHit?)
        (bind _corner (Utilities|GetCorner)
          (:IsInCorner
            (bind _asbp_corner_index (Utilities|Casting|CastToBP_CornerIndex _corner))
            (switch Utilities|FlowControl|Switch|SwitchonE_Turnindex (Variables|/Game/VehicleAdvBP/Blueprints/Car_AI/BP_CornerIndex.BP_CornerIndex_C|GetTurnIndex _asbp_corner_index)
              (:NewEnumerator0
                (Utilities|SpeedLimit 3e+01
                  (:Under%20Speed%20Limit
                    (CallFunction|SetInput 1.0 0.0))
                  (:Over%20Speed%20Limit
                    (CallFunction|SetInput 0.0 1.0))))
              (:NewEnumerator1
                (Utilities|SpeedLimit 12.0
                  (:Under%20Speed%20Limit
                    (CallFunction|SetInput 1.0 0.0))
                  (:Over%20Speed%20Limit
                    (CallFunction|SetInput 0.0 1.0))))))
          (:NoInCorner
            (CallFunction|SetInput 0.0 (Math|Float|MapRangeClamped (.distance (Variables|Default|GetFrontLineTraceHitResult)) 0.0 1.0 0.0 1.5e+03))))
        (else
          (CallFunction|SetInput 1.0 0.0))))))

(fn ConstructionScript)

(fn GetPath
  (params (Splines :type Array%20of%20Path%202%20Object%20References))
  (bind _returnvalue (Transformation|GetActorLocation))
  (bind _output (Utilities|Array|Get(acopy) Splines))
  (bind _spline (Variables|/Game/VehicleAdvBP/Blueprints/Car_AI/Path2.Path2_C|GetSpline _output))
  (return (Math|Float|MapRangeClamped (.yaw (Math|Rotator|Delta(Rotator) (Math|Rotator|FindLookatRotation _returnvalue (Spline|FindLocationClosesttoWorldLocation _spline (+ (* (Math|Vector|Normalize (Class|SplineComponent|FindTangentClosesttoWorldLocation _spline _returnvalue "World")) (Math|Float|MapRangeClamped (CallFunction|GetCurrentCarSpeed) 2e+01 8e+01 5e+01 5e+02)) _returnvalue) "World")) (Transformation|GetActorRotation))) -9e+01 9e+01 -1.0 1.0)))

(fn GetCurrentCarSpeed
  (return (* (Class|WheeledVehicleMovementComponent|GetForwardSpeed (Variables|Default|GetVehicleMovement)) 0.036)))

(fn SetInput
  (params (Throttle :type Float%20%28single-precision%29) (Brake :type Float%20%28single-precision%29))
  (bind _vehiclemovement (Variables|Default|GetVehicleMovement))
  (Class|WheeledVehicleMovementComponent|SetThrottleInput _vehiclemovement Throttle)
  (Class|WheeledVehicleMovementComponent|SetBrakeInput _vehiclemovement Brake))

(fn LineTracer
  (bind _linetracestartpoint (Variables|Default|GetLineTraceStartPoint))
  (bind _returnvalue (Transformation|GetWorldLocation _linetracestartpoint))
  (bind (_outhit _returnvalue_2) (Collision|LineTraceByChannel _returnvalue (+ _returnvalue (* (Math|Vector|GetForwardVector _linetracestartpoint) 8e+02)) "TraceTypeQuery1" false 0 "ForOneFrame"))
  (Variables|Default|SetFrontLineTraceHitResult _outhit)
  (Variables|Default|SetFrontLineTraceHit? _returnvalue_2))