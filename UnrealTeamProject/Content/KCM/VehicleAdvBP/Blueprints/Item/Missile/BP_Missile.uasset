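; Homing missile projectile that explodes on first impact in what appears to be a vehicle combat game.
; HomingMissile attaches a scene component to the given target and makes the projectile movement home on it.
; On hit it fires a radial impulse, spawns an explosion and destroys itself.
; Two identical branches then unlock the first AI4 vehicle's mesh constraint, with an XY-plane relock delayed after the destroy call.
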(event OnComponentHit(CollisionComponent)
  (params (HitComponent :type Primitive%20Component%20Object%20Reference) (OtherActor :type Actor%20Object%20Reference) (OtherComp :type Primitive%20Component%20Object%20Reference) (NormalImpulse :type Vector :default "0, 0, 0") (Hit :type Hit%20Result%20Structure%20%28by%20ref%29))
  (bind _explosionforce (Variables|Default|GetExplosionForce))
  ;[0 0 0] Bomb
  (Utilities|FlowControl|DoOnce false
    (:Completed
      (Class|RadialForceComponent|FireImpulse _explosionforce)
      (Effects|SpawnEmitteratLocation "/Game/StarterContent/Particles/P_Explosion.P_Explosion" (Transformation|GetWorldLocation _explosionforce))
      (Actor|DestroyActor)
      (Utilities|FlowControl|Sequence
        (:then_0
          (bind _outactors (Actor|GetAllActorsOfClass "/Game/HCH/VehicleAdvBP/Blueprints/Car_AI/BP_VehicleBlueprint_AI4.BP_VehicleBlueprint_AI4_C"))
          (Class|PrimitiveComponent|SetConstraintMode (Variables|/Script/PhysXVehicles.WheeledVehicle|GetMesh (Utilities|Array|Get(acopy) _outactors)) "None")
          (Utilities|FlowControl|Delay 2.0)
          (Class|PrimitiveComponent|SetConstraintMode (Variables|/Script/PhysXVehicles.WheeledVehicle|GetMesh (Utilities|Array|Get(acopy) _outactors)) "XYPlane"))
        (:then_1
          (bind _outactors_2 (Actor|GetAllActorsOfClass "/Game/HCH/VehicleAdvBP/Blueprints/Car_AI/BP_VehicleBlueprint_AI4.BP_VehicleBlueprint_AI4_C"))
          (Class|PrimitiveComponent|SetConstraintMode (Variables|/Script/PhysXVehicles.WheeledVehicle|GetMesh (Utilities|Array|Get(acopy) _outactors_2)) "None")
          (Utilities|FlowControl|Delay 2.0)
          (Class|PrimitiveComponent|SetConstraintMode (Variables|/Script/PhysXVehicles.WheeledVehicle|GetMesh (Utilities|Array|Get(acopy) _outactors_2)) "XYPlane"))))))

(event Custom|HomingMissile
  (params (TargetToHit :type Wheeled%20Vehicle%20Object%20Reference))
  (bind _projectile (Variables|MyProjectile|GetProjectile))
  ;[0 0 0] Set Homing Missile
  (bind _returnvalue (AddComponent|AddSceneComponent TargetToHit false))
  (if (Utilities|IsValid TargetToHit)
    (Variables|/Script/Engine.ProjectileMovementComponent|SetHomingTargetComponent _projectile _returnvalue)
    (Variables|/Script/Engine.ProjectileMovementComponent|SetbIsHomingProjectile _projectile true)
    (Variables|/Script/Engine.ProjectileMovementComponent|SetHomingAccelerationMagnitude _projectile 2.5e+04)))

(fn ConstructionScript)